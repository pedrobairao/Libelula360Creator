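; BP_ActionFunction executes scene interaction actions passed to DoAction as a transform and action struct, dispatching by action type.
; Door starts a fade-out sequence, stores the next scene ID in the AppContext game instance and immediately opens the Scene level.
; Audio plays a 2D sound only once, as its Playing flag never resets.
; Text spawns a BP_TextAction at the given transform, rotated toward the player.
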(event `DoAction`
  (params (Position :type "Transform Structure") (Action_Struct :type "/Game/SaveSettings/Action_Struct Structure (by ref)"))
  (set `self.Position` Position)
  (bind _output_get (set `self.Action` Action_Struct))
  (switch `string` (`.ActionType_25_3AE1B14948ABD39F2DA39F938ADA3CC6` (break `/Game/SaveSettings/Action_Struct` _output_get))
    (:`Door`
      (`self.Door`))
    (:`Audio`
      (`self.Audio`))
    (:`Text`
      (`self.Text`))))

(fn `Audio`
  (if (not (`self.Playing`))
    (`GameplayStatics.PlaySound2D` (`.Sound_22_B472F9AE4668A90127A95798B71C64C7` (break `/Game/SaveSettings/Action_Struct` (`self.Action`))) 1.0 1.0 0.0 null null)
    (set `self.Playing` true)))

(fn `Door`
  (bind _outactor (`LevelSequencePlayer.CreateLevelSequencePlayer` "/Game/Assets/Sequences/FadeOut_Sequence/FadeOut_SequenceMaster.FadeOut_SequenceMaster"))
  (`MovieSceneSequencePlayer.Play` (`LevelSequenceActor.SequencePlayer` _outactor))
  (bind _asapp_context (cast `/Game/SaveSettings/AppContext` (`GameplayStatics.GetGameInstance`)))
  (set `/Game/SaveSettings/AppContext.CurrentSceneID` (`.NextScene_14_C513758F467CE5D13E936899011A1634` (break `/Game/SaveSettings/Action_Struct` (`self.Action`))) _asapp_context)
  (`GameplayStatics.OpenLevel` "Scene"))

(fn `Text`
  (bind _returnvalue (`|SpawnActorFromClass` "/Game/Blueprints/BP_TextAction.BP_TextAction_C" (`KismetMathLibrary.MakeTransform` (.location (`self.Position`)) (.rotation (`self.Position`))) "Undefined" "OverrideRootScale" null null))
  (bind _textrender (`/Game/Blueprints/BP_TextAction.TextRender` _returnvalue))
  (`TextRenderComponent.K2_SetText` _textrender (`|FormatText` (`.Text_28_45AB27D040B8E2D2EB8E228186667E5E` (break `/Game/SaveSettings/Action_Struct` (`self.Action`))) (`self.linebreak`)))
  (`SceneComponent.K2_SetWorldRotation` _textrender (`KismetMathLibrary.FindLookAtRotation` (.location (`self.Position`)) (`Actor.K2_GetActorLocation` (`GameplayStatics.GetPlayerPawn` 0))) false false))